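; Player controller for the main menu, handling game start, quit and a donate link.
; On BeginPlay it shows W_MainMenu, sets game-only input and turns off shadows through console commands.
; Releasing Enter triggers StartGame once via a guard flag; start and quit both hide the widget and wait briefly before loading LVL_Game or exiting.
; The Donate input opens the stored URL if it can be launched.
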(event `self.ReceiveBeginPlay`
  (bind _returnvalue (`|CreateWidget` "/Game/GirlKnight/Core/UI/W_MainMenu.W_MainMenu_C" self))
  (`UserWidget.AddToViewport` _returnvalue 0)
  (set `self.MenuWidget` _returnvalue)
  (`WidgetBlueprintLibrary.SetInputMode_GameOnly` self)
  (`KismetSystemLibrary.ExecuteConsoleCommand` "r.DynamicShadows 0" null)
  (`KismetSystemLibrary.ExecuteConsoleCommand` "r.ShadowQuality 0" null))

(event `StartGame`
  (`/Game/GirlKnight/Core/UI/W_MainMenu.HideWidget` (`self.MenuWidget`))
  (`KismetSystemLibrary.Delay` 0.5)
  (`GameplayStatics.OpenLevel` "LVL_Game"))

(event `QuitGame`
  (`/Game/GirlKnight/Core/UI/W_MainMenu.HideWidget` (`self.MenuWidget`))
  (`KismetSystemLibrary.Delay` 0.5)
  (`KismetSystemLibrary.QuitGame` null "Quit"))

(event `InputAction|Enter`
  (params (Key :type "Key Structure"))
  (:`Released`
    (if (not (`self.bEnteringToGame`))
      (set `self.bEnteringToGame` true)
      (`self.StartGame`))))

(event `InputAction|Donate`
  (params (Key :type "Key Structure"))
  (:`Pressed`
    (bind _returnvalue (`KismetSystemLibrary.CanLaunchURL` (`self.Url`)))
    (if _returnvalue
      (`KismetSystemLibrary.LaunchURL` (`self.Url`)))))

(fn `UserConstructionScript`)
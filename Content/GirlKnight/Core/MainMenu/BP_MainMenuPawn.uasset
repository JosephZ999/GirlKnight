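; Main menu pawn that moves steadily along X to scroll a parallax sprite background.
; On BeginPlay it gives each Paper sprite under Backgrounds a dynamic material instance with a parallax multiplier matched by child index.
; Every tick it offsets the actor by walk speed, then passes the camera's world X to those materials, leaving the parallax effect to the material.
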(event `self.ReceiveBeginPlay`
  (for (_array_element _array_index) (`SceneComponent.GetChildrenComponents` (`self.Backgrounds`) false)
    (bind _aspaper_sprite_component (cast `PaperSpriteComponent` _array_element))
    (bind _returnvalue (`PrimitiveComponent.CreateDynamicMaterialInstance` _aspaper_sprite_component 0 "/Game/GirlKnight/Materials/MI_BackgroundSprite.MI_BackgroundSprite" "None"))
    (`MaterialInstanceDynamic.SetScalarParameterValue` _returnvalue "ParallaxMultiplier" (`|GetArrayItem` (`self.ParrallaxMultipliers`) _array_index))
    (`KismetArrayLibrary.Array_Add` (`self.BackgroundMaterials`) _returnvalue)))

(event `UpdateBgPos`
  (for _array_element (`self.BackgroundMaterials`)
    (`MaterialInstanceDynamic.SetScalarParameterValue` _array_element "CameraX" (.x (`SceneComponent.K2_GetComponentLocation` (`self.Camera`))))))

(event `self.ReceiveTick`
  (params (DeltaSeconds :type "Float (single-precision)"))
  (`self.K2_AddActorWorldOffset` (`KismetMathLibrary.MakeVector` (* DeltaSeconds (`self.PlayerWalkSpeed`))) true)
  (`self.UpdateBgPos`))

(fn `UserConstructionScript`)
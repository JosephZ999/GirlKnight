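; BP_PlayerPawn is the moving stage of a side-scrolling battler, spawning and animating the knight, goblins and wave chest.
; It walks along X on Tick, feeding camera X to dynamic background sprite materials for parallax.
; Each enemy spawns ahead, and a timed delay stops the walk and signals the encounter.
; Events play attacks with hit-timed reactions and sound, deaths, and the chest opening on wave win.
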(event `self.ReceiveBeginPlay`
  ;[1 1 1] Background
  (for (_array_element _array_index) (`SceneComponent.GetChildrenComponents` (`self.Backgrounds`) false)
    (bind _aspaper_sprite_component (cast `PaperSpriteComponent` _array_element))
    (bind _returnvalue (`PrimitiveComponent.CreateDynamicMaterialInstance` _aspaper_sprite_component 0 "/Game/GirlKnight/Materials/MI_BackgroundSprite.MI_BackgroundSprite" "None"))
    (`MaterialInstanceDynamic.SetScalarParameterValue` _returnvalue "ParallaxMultiplier" (`|GetArrayItem` (`self.ParrallaxMultipliers`) _array_index))
    (`KismetArrayLibrary.Array_Add` (`self.BackgroundMaterials`) _returnvalue)))

(event `UpdateBgPos`
  ;[1 1 1] Background
  (for _array_element (`self.BackgroundMaterials`)
    (`MaterialInstanceDynamic.SetScalarParameterValue` _array_element "CameraX" (.x (`SceneComponent.K2_GetComponentLocation` (`self.Camera`))))))

(event `self.ReceiveTick`
  (params (DeltaSeconds :type "Float (single-precision)"))
  (if (`self.Walking`)
    (`self.K2_AddActorWorldOffset` (`KismetMathLibrary.MakeVector` (* DeltaSeconds (`self.PlayerWalkSpeed`))) true)
    (`self.UpdateBgPos`)))

(event `SpawnPlayerCharacter`
  (bind _returnvalue (`|SpawnActorFromClass` "/Game/GirlKnight/Core/Game/Characters/BP_PlayerChar.BP_PlayerChar_C" (`KismetMathLibrary.MakeTransform` (`SceneComponent.K2_GetComponentLocation` (`self.PlayerPos`))) "AlwaysSpawn" "OverrideRootScale" null null))
  (set `self.PlayerCharacter` _returnvalue)
  (`self.K2_AttachToActor` _returnvalue self "None" "KeepWorld" "KeepWorld" "KeepRelative" false)
  (`self.Walk` true))

(event `SpawnEnemy`
  (bind _enemycharacter (`self.EnemyCharacter`))
  (`self.Walk` true)
  (`/Engine/EditorBlueprintResources/StandardMacros.IsValid` _enemycharacter
    (:`Is Valid`
      (`self.SetLifeSpan` _enemycharacter 5.0))
    (:`Is Not Valid`
      _))
  (bind _returnvalue (`|SpawnActorFromClass` "/Game/GirlKnight/Core/Game/Characters/BP_GoblinChar.BP_GoblinChar_C" (`KismetMathLibrary.MakeTransform` (+ (`SceneComponent.K2_GetComponentLocation` (`self.PlayerPos`)) (`KismetMathLibrary.MakeVector` (`self.EnemyDist`))) (struct :`Yaw` 180.0)) "AlwaysSpawn" "OverrideRootScale" null null))
  (set `self.EnemyCharacter` _returnvalue)
  (`KismetSystemLibrary.Delay` (/ (- (`self.EnemyDist`) 200.0) (`self.PlayerWalkSpeed`)))
  (`self.Walk` false)
  (`self.EnemyFound`))

(event `EnemyAttack`
  (bind _enemycharacter (`self.EnemyCharacter`))
  (`/Game/GirlKnight/Core/Game/BP_Character.Attack` _enemycharacter)
  (bind _time (`/Game/GirlKnight/Core/Game/BP_Character.GetHitTime` _enemycharacter))
  (`KismetSystemLibrary.Delay` _time)
  (`/Game/GirlKnight/Core/Game/BP_Character.Hit` (`self.PlayerCharacter`))
  (`GameplayStatics.PlaySound2D` "/Game/GirlKnight/Sounds/SFX_Attack.SFX_Attack" 1.0 1.0 0.0 null null :!label _label))

(event `PlayerAttack`
  (bind _playercharacter (`self.PlayerCharacter`))
  (`/Game/GirlKnight/Core/Game/BP_Character.Attack` _playercharacter)
  (bind _time (`/Game/GirlKnight/Core/Game/BP_Character.GetHitTime` _playercharacter))
  (`KismetSystemLibrary.Delay` _time)
  (`/Game/GirlKnight/Core/Game/BP_Character.Hit` (`self.EnemyCharacter`))
  (goto _label))

(event `PlayerDeath`
  (`/Game/GirlKnight/Core/Game/BP_Character.Fall` (`self.PlayerCharacter`)))

(event `EnemyDeath`
  (`/Game/GirlKnight/Core/Game/BP_Character.Fall` (`self.EnemyCharacter`)))

(event `OnLastEnemySpawn`
  ;[1 1 1] Chest
  (bind _returnvalue (`|SpawnActorFromClass` "/Game/GirlKnight/Core/Game/Characters/BP_Chest.BP_Chest_C" (`KismetMathLibrary.MakeTransform` (+ (`SceneComponent.K2_GetComponentLocation` (`self.PlayerPos`)) (`KismetMathLibrary.MakeVector` (+ (`self.EnemyDist`) 100.0)))) "Undefined" "OverrideRootScale" null null))
  (set `self.ChestActor` _returnvalue))

(event `OnWaveWin`
  ;[1 1 1] Chest
  (`KismetSystemLibrary.Delay` 1.0)
  (`/Engine/EditorBlueprintResources/StandardMacros.IsValid` (`self.ChestActor`)
    (:`Is Valid`
      (`/Game/GirlKnight/Core/Game/Characters/BP_Chest.Open` (`self.ChestActor`)))))

(fn `Attack`
  (params (Attacker :type "/Game/GirlKnight/Core/Game/BP_Character Object Reference") (Victim :type "/Game/GirlKnight/Core/Game/BP_Character Object Reference")))

(fn `UserConstructionScript`)

(fn `Walk`
  (params (Enabled :type Boolean))
  (bind _output_get (set `self.Walking` Enabled))
  (if _output_get
    (`/Game/GirlKnight/Core/Game/BP_Character.Walk` (`self.PlayerCharacter`))
    (else
      (`/Game/GirlKnight/Core/Game/BP_Character.Stand` (`self.PlayerCharacter`)))))
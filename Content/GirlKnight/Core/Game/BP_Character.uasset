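; Flipbook-animated character Blueprint that exposes Stand, Walk, Attack, Hit and Fall events to drive a 2D sprite.
; Each event plays its animation through PlayAnim, with retriggerable delays returning Attack and Hit to idle.
; Attack picks a random animation and, after a delay, offsets the sprite along X with a timeline dash.
; Fall only sets a flag, so the next Hit to finish plays the fall animation and death sound.
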(event `self.ReceiveBeginPlay`
  (`self.Stand`))

(event `Stand`
  (`self.PlayAnim` (`self.IdleAnim`) true))

(event `Attack`
  (bind _attackindex (`self.AttackIndex`))
  (bind _attackanims (`self.AttackAnims`))
  (`|ExecutionSequence`
    (:`then_0`
      (set `self.AttackIndex` (`KismetMathLibrary.RandomInteger` (- (`KismetArrayLibrary.Array_Length` (`self.AttackAnims`)) 1)))
      (if (`KismetArrayLibrary.Array_IsValidIndex` _attackanims _attackindex)
        (`self.PlayAnim` (`|GetArrayItem` _attackanims _attackindex) false true)
        (`KismetSystemLibrary.RetriggerableDelay` (`PaperFlipbook.GetTotalDuration` (`|GetArrayItem` (`self.AttackAnims`) (`self.AttackIndex`))))
        (`self.Stand`)))
    (:`then_1`
      (`KismetSystemLibrary.Delay` (`self.AttackDashDelay`))
      (bind (_direction _scalar) (`Timeline|AttackDash` :!via `PlayFromStart`)
        (:`Update`
          (`SceneComponent.K2_SetRelativeLocation` (`self.Sprite`) (* (`KismetMathLibrary.MakeVector` 1.0) (* 50.0 _scalar)) false false))))))

(event `Walk`
  (`self.PlayAnim` (`self.WalkAnim`) true))

(event `Hit`
  (`self.PlayAnim` (`self.HitAnim`) false true)
  (`KismetSystemLibrary.RetriggerableDelay` (`PaperFlipbook.GetTotalDuration` (`self.HitAnim`)))
  (if (`self.MustFall`)
    (`self.PlayAnim` (`self.FallAnim`) false true)
    (`GameplayStatics.PlaySound2D` (`self.DeathSound`) 1.0 1.0 0.0 null null)
    (else
      (`self.Stand`))))

(event `Fall`
  (set `self.MustFall` true))

(fn `GetHitTime`
  (returns (Time :type "Float (double-precision)"))
  (return 0.5))

(fn `PlayAnim`
  (params (InAnim :type "PaperFlipbook Object Reference") (bLoop :type Boolean) (bPlayFromStart :type Boolean))
  (bind _sprite (`self.Sprite`))
  (`PaperFlipbookComponent.SetFlipbook` (`self.Sprite`) InAnim)
  (`PaperFlipbookComponent.SetLooping` (`self.Sprite`) bLoop)
  (if bPlayFromStart
    (`PaperFlipbookComponent.PlayFromStart` _sprite)
    (else
      (`PaperFlipbookComponent.Play` _sprite))))

(fn `UserConstructionScript`)
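; Player controller that drives the battle loop, relaying game events to the player pawn and HUD.
; On begin play it caches BP_PlayerPawn and binds its enemy-found callback to start a battle.
; Spawn, attack and death events forward to the pawn, while battle events toggle the game UI and a win spawns the next enemy after a short delay.
; Right and wrong player actions play feedback sounds; wave win is an empty stub.
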(event `self.ReceiveBeginPlay`
  (bind _asbp_player_pawn (cast `/Game/GirlKnight/Core/Game/BP_PlayerPawn` (`GameplayStatics.GetPlayerPawn` 0)))
  (bind _output_get (set `self.PawnPtr` _asbp_player_pawn))
  (add `/Game/GirlKnight/Core/Game/BP_PlayerPawn.EnemyFound` _output_get (delegate `EnemyFound`))
  (`WidgetBlueprintLibrary.SetInputMode_GameOnly` self))

(event `EnemyFound`
  (`self.StartBattle`))

(event `self.OnPlayerSpawn`
  (params (InCharIndex :type "Name (by ref)"))
  (`/Game/GirlKnight/Core/Game/BP_PlayerPawn.SpawnPlayerCharacter` (`self.PawnPtr`)))

(event `self.OnBattleStart`
  ;[1 1 1] Main
  (bind _asbp_game_hud (cast `/Game/GirlKnight/Core/Game/BP_GameHUD` (`self.GetHUD`)))
  (`/Game/GirlKnight/Core/Game/BP_GameHUD.ToggleGameUI` _asbp_game_hud true)
  (`KismetSystemLibrary.PrintString` "Hello"))

(event `self.OnEnemySpawn`
  (params (InCharIndex :type "Name (by ref)"))
  (`/Game/GirlKnight/Core/Game/BP_PlayerPawn.SpawnEnemy` (`self.PawnPtr`)))

(event `self.OnGameStart`
  ;[1 1 1] Main
  (`self.SpawnEnemy`))

(event `self.OnEnemyAttack`
  (params (InAttackParam :type "GK_AttackData Structure (by ref)"))
  (`/Game/GirlKnight/Core/Game/BP_PlayerPawn.EnemyAttack` (`self.PawnPtr`)))

(event `self.OnBattleFail`
  ;[1 1 1] Main
  (bind _asbp_game_hud (cast `/Game/GirlKnight/Core/Game/BP_GameHUD` (`self.GetHUD`)))
  (`/Game/GirlKnight/Core/Game/BP_GameHUD.ToggleGameUI` _asbp_game_hud false))

(event `self.OnPlayerAttack`
  (params (InAttackParam :type "GK_AttackData Structure (by ref)"))
  (`/Game/GirlKnight/Core/Game/BP_PlayerPawn.PlayerAttack` (`self.PawnPtr`)))

(event `self.OnBattleWin`
  ;[1 1 1] Main
  (bind _asbp_game_hud (cast `/Game/GirlKnight/Core/Game/BP_GameHUD` (`self.GetHUD`)))
  (`/Game/GirlKnight/Core/Game/BP_GameHUD.ToggleGameUI` _asbp_game_hud false)
  (`KismetSystemLibrary.Delay` 1.0)
  (`self.SpawnEnemy`))

(event `self.OnEnemyDead`
  (`/Game/GirlKnight/Core/Game/BP_PlayerPawn.EnemyDeath` (`self.PawnPtr`)))

(event `self.OnWaveWin`
  ;[1 1 1] Main
)

(event `self.OnPlayerDead`
  (`/Game/GirlKnight/Core/Game/BP_PlayerPawn.PlayerDeath` (`self.PawnPtr`)))

(event `self.OnRightAction`
  ;[1 1 1] Player Actions
  (`GameplayStatics.PlaySound2D` "/Game/GirlKnight/Sounds/Confirm_1.Confirm_1" 1.0 1.0 0.0 null null))

(event `self.OnWrongAction`
  ;[1 1 1] Player Actions
  (`GameplayStatics.PlaySound2D` "/Game/GirlKnight/Sounds/Block_Break_1.Block_Break_1" 1.0 1.0 0.0 null null))

(fn `UserConstructionScript`)
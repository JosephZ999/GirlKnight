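; BP_GameHUD is the game HUD Blueprint that owns the main game UI widget and toggles its visibility.
; InitWidget lazily creates the widget from GameUIClass, adds it to the viewport and caches it in GameUIWidget for reuse.
; ToggleGameUI gets the widget through InitWidget, then calls its Show or Hide function based on the Show flag.
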(fn `InitWidget`
  (returns (GameUIWidget :type "/Game/GirlKnight/Core/UI/W_GameUI Object Reference"))
  (`/Engine/EditorBlueprintResources/StandardMacros.IsValid` (`self.GameUIWidget`)
    (:`Is Valid`
      (return (`self.GameUIWidget`)))
    (:`Is Not Valid`
      (bind _returnvalue (`|CreateWidget` (`self.GameUIClass`)))
      (bind _output_get (set `self.GameUIWidget` _returnvalue))
      (`UserWidget.AddToViewport` _output_get 0)
      (return (`self.GameUIWidget`)))))

(fn `ToggleGameUI`
  (params (Show :type Boolean))
  (bind _gameuiwidget (`self.InitWidget`))
  (if Show
    (`/Game/GirlKnight/Core/UI/W_GameUI.Show` _gameuiwidget)
    (else
      (`/Game/GirlKnight/Core/UI/W_GameUI.Hide` _gameuiwidget))))

(fn `UserConstructionScript`)